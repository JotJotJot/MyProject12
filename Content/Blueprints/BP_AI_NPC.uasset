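; Voice-driven AI NPC Blueprint that turns recorded player speech into an OpenAI chat reply.
; Start and stop events drive audio capture and submix recording to a WAV file, whose completion triggers OpenAI transcription.
; The transcript becomes a user message for a GPT-3.5 Turbo call, with both sides logged and appended to a chat log.
; Replies go to ContextDetection, which is still an empty stub.
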(event `self.ReceiveBeginPlay`
  (`OpenAIUtils.setUseOpenAIApiKeyFromEnvironmentVars` true))

(event `StartRecording`
  (`SynthComponent.Start` (`self.AudioCapture`))
  (`KismetSystemLibrary.PrintString` "Start")
  (`AudioMixerBlueprintLibrary.StartRecordingOutput` 0.0 (`self.MySubmix`)))

(event `StopRecording`
  (`SynthComponent.Stop` (`self.AudioCapture`))
  (`AudioMixerBlueprintLibrary.StopRecordingOutput` "WavFile" (`self.FileName`) "" (`self.MySubmix`) null)
  (add `SoundSubmix.OnSubmixRecordedFileDone` (`self.MySubmix`) (delegate `SoundToText`)))

(event `SoundToText`
  (params (ResultingSoundWave :type "SoundWave Object Reference"))
  (`KismetSystemLibrary.PrintString` "Konwertuje")
  (bind (_transcription _errormessage _success) (`OpenAICallTranscriptions.OpenAICallTranscriptions` (`self.FileName`))
    (:`Finished`
      (if _success
        (`KismetSystemLibrary.LogString` (`KismetStringLibrary.Concat_StrStr` "USER: " _transcription))
        (`self.SendPrompt` (make `ChatLog` "USER" _transcription))
        (else
          (`KismetSystemLibrary.PrintString` _errormessage))))))

(event `SendPrompt`
  (params (ChatLog :type "ChatLog Structure"))
  (`KismetArrayLibrary.Array_Add` (`self.ChatLog`) ChatLog)
  (bind (_message _errormessage _success) (`OpenAICallChat.OpenAICallChat` (make `ChatSettings` :`model` "GPT_3_5_TURBO" :`temperature` 0.7 :`maxTokens` 150))
    (:`Finished`
      (if _success
        (bind _message_2 (break `ChatCompletion` _message))
        (`KismetArrayLibrary.Array_Add` (`self.ChatLog`) _message_2)
        (bind (_role _content) (break `ChatLog` _message_2))
        (`KismetSystemLibrary.LogString` (`KismetStringLibrary.Concat_StrStr` "ASSISTANT: " _content))
        (`self.ContextDetection` _content)
        (else
          (`KismetSystemLibrary.PrintString` _errormessage))))))

(fn `ContextDetection`
  (params (Content :type String)))

(fn `UserConstructionScript`)